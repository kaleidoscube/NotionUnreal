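; BP_Notion_GlobalFunctions provides global helper functions for setting, clearing and saving named Notion task properties.
; All of them go through GetNotionSaveData, which finds BP_Notion_SaveManager on player controller 0, adding and initializing it on first use.
; Property edits change the manager's in-memory map; persistence across sessions happens only through SaveNotionPropertiesAccrossSessions, which ClearNotionProperties can optionally invoke.
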(fn SetNotionTaskProperty
  (params (PropertyName :type String) (Value :type String))
  (bind ___worldcontext (LocalVariables|Get__WorldContext))
  (bind _returnvalue (NotionUnreal|GetNotionSaveData ___worldcontext))
  (bind _propertysavedata (Variables|/NotionUnreal/BP_Notion_SaveManager.BP_Notion_SaveManager_C|GetPropertySaveData _returnvalue))
  (LocalVariables|SetProperty PropertyName)
  (LocalVariables|SetVal Value)
  (LocalVariables|SetSaveProperties (Variables|/NotionUnreal/BP_Notion_SaveData.BP_Notion_SaveData_C|GetProperties _propertysavedata))
  (if (Utilities|Map|Contains (LocalVariables|GetSaveProperties) (LocalVariables|GetProperty))
    (Utilities|Map|Remove (LocalVariables|GetSaveProperties) (LocalVariables|GetProperty)))
  (Utilities|Map|Add (LocalVariables|GetSaveProperties) (LocalVariables|GetProperty) (LocalVariables|GetVal))
  (Variables|/NotionUnreal/BP_Notion_SaveData.BP_Notion_SaveData_C|SetProperties _propertysavedata (LocalVariables|GetSaveProperties)))

(fn GetNotionSaveData
  (bind ___worldcontext (LocalVariables|Get__WorldContext))
  (bind _returnvalue (Game|GetPlayerController ___worldcontext))
  (Utilities|IsValid ___worldcontext
    (:Is%20Valid
      (Utilities|IsValid _returnvalue
        (:Is%20Valid
          (Utilities|IsValid (Actor|GetComponentbyClass _returnvalue "/NotionUnreal/BP_Notion_SaveManager.BP_Notion_SaveManager_C")
            (:Is%20Valid
              _)
            (:Is%20Not%20Valid
              (bind _returnvalue_2 (Game|AddComponentbyClass _returnvalue "/NotionUnreal/BP_Notion_SaveManager.BP_Notion_SaveManager_C"))
              (Default|Init _returnvalue_2)))
          (return (Actor|GetComponentbyClass (Game|GetPlayerController (LocalVariables|Get__WorldContext)) "/NotionUnreal/BP_Notion_SaveManager.BP_Notion_SaveManager_C") true))
        (:Is%20Not%20Valid
          _)))
    (:Is%20Not%20Valid
      _))
  (return 0 false))

(fn SaveNotionPropertiesAccrossSessions
  (bind ___worldcontext (LocalVariables|Get__WorldContext))
  (bind (_returnvalue _sucess) (NotionUnreal|GetNotionSaveData ___worldcontext))
  (if _sucess
    (Default|SavePropertyData _returnvalue)))

(fn ClearNotionProperties
  (params (SaveAccrossSessions :type Boolean))
  (Utilities|Map|Clear (Variables|/NotionUnreal/BP_Notion_SaveData.BP_Notion_SaveData_C|GetProperties (Variables|/NotionUnreal/BP_Notion_SaveManager.BP_Notion_SaveManager_C|GetPropertySaveData (.ReturnValue (NotionUnreal|GetNotionSaveData (LocalVariables|Get__WorldContext))))))
  (if SaveAccrossSessions
    (NotionUnreal|SaveNotionPropertiesAccrossSessions (LocalVariables|Get__WorldContext))))

(fn ClearNotionProperty
  (params (PropertyName :type String))
  (bind ___worldcontext (LocalVariables|Get__WorldContext))
  (bind _returnvalue (NotionUnreal|GetNotionSaveData ___worldcontext))
  (bind _propertysavedata (Variables|/NotionUnreal/BP_Notion_SaveManager.BP_Notion_SaveManager_C|GetPropertySaveData _returnvalue))
  (LocalVariables|SetSaveProperties (Variables|/NotionUnreal/BP_Notion_SaveData.BP_Notion_SaveData_C|GetProperties _propertysavedata))
  (if (Utilities|Map|Contains (LocalVariables|GetSaveProperties) PropertyName)
    (Utilities|Map|Remove (LocalVariables|GetSaveProperties) PropertyName)
    (Variables|/NotionUnreal/BP_Notion_SaveData.BP_Notion_SaveData_C|SetProperties _propertysavedata (LocalVariables|GetSaveProperties))))